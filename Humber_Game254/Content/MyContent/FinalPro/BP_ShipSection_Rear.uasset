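; BP_ShipSection_Rear is the rear section of a ship, with body, connector, accent and thruster components.
; ChangeMat applies a body material to the main body and a shared accent material to the connector and accent.
; ResizeThruster sets the thruster's world-space Z scale in proportion to a given speed, keeping X and Y unchanged.
; BeginPlay and construction only defer to the parent, and Tick is disabled.
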(event `self.ReceiveBeginPlay`
  (`parent.ReceiveBeginPlay`))

(event `self.ChangeMat`
  (params (NewBodyMat :type "MaterialInstance Object Reference") (NewAccentMat :type "MaterialInstance Object Reference"))
  (`PrimitiveComponent.SetMaterial` (`self.MainBody`) 0 NewBodyMat)
  (`PrimitiveComponent.SetMaterial` (`self.Connector`) 0 NewAccentMat)
  (`PrimitiveComponent.SetMaterial` (`self.Accent`) 0 NewAccentMat))

(fn `ResizeThruster`
  (params (Speed :type "Float (double-precision)"))
  (`SceneComponent.SetWorldScale3D` (`self.Thruster`) (`KismetMathLibrary.MakeVector` (.x (.scale (`SceneComponent.K2_GetComponentToWorld` (`self.Thruster`)))) (.y (.scale (`SceneComponent.K2_GetComponentToWorld` (`self.Thruster`)))) (/ Speed 4.0))))

(fn `UserConstructionScript`
  (`parent.UserConstructionScript`))