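; Modular spaceship actor that builds its hull at runtime from separately spawned section actors.
; On BeginPlay, InitShip spawns basic sections based on ShipLength, placing each at the previous one's rear attach location, then caps the chain with a rear section.
; SetShipsMat applies body and accent materials to the stored sections, Helm and Connector.
; Tick passes Speed to the last section to resize its thruster.
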(event `self.ReceiveBeginPlay`
  (`self.InitShip`))

(event `self.ReceiveTick`
  (params (DeltaSeconds :type "Float (single-precision)"))
  (bind _shipsegmentarray (`self.ShipSegmentArray`))
  ;[0 1 0.1265] Change Thruster Size based on speed
  (bind _asbp_ship_section_rear (cast `/Game/MyContent/FinalPro/BP_ShipSection_Rear` (`|GetArrayItem` _shipsegmentarray (`KismetArrayLibrary.Array_LastIndex` _shipsegmentarray))))
  (`/Game/MyContent/FinalPro/BP_ShipSection_Rear.ResizeThruster` _asbp_ship_section_rear (`self.Speed`)))

(fn `InitShip`
  (locals (TargetLocation :type "Vector Structure"))
  (bind _shipsegmentarray (`self.ShipSegmentArray`))
  (bind _returnvalue (`KismetMathLibrary.MakeTransform` (`local.TargetLocation`)))
  ;[1 1 1] Grab First Spawn Location
  (set `local.TargetLocation` (`SceneComponent.K2_GetComponentLocation` (`self.Connection`)))
  ;[1 1 1] For Ships length spawn sections and finish with rear section
  (for _ (range (+ (`self.ShipLength`) 1))
    (bind _returnvalue_2 (`|SpawnActorFromClass` "/Game/MyContent/FinalPro/BP_ShipSection_Basic.BP_ShipSection_Basic_C" _returnvalue "Undefined" "OverrideRootScale" null null))
    ;[1 1 1] Add Ship Sections to Array
    (`KismetArrayLibrary.Array_Add` _shipsegmentarray _returnvalue_2)
    ;[1 1 1] Set TargetLocation to next segment
    (bind _asbp_ship_section_master (cast `/Game/MyContent/FinalPro/BP_ShipSection_Master` _returnvalue_2))
    (bind _transform (`/Game/MyContent/FinalPro/BP_ShipSection_Master.GetRearAttachTransform` _asbp_ship_section_master))
    (set `local.TargetLocation` (.location _transform))
    ;[1 1 1] Set Segment Colors
    (`self.SetShipsMat` (`self.M_Body`) (`self.M_Accent`) :!label _label))
  (bind _returnvalue_3 (`|SpawnActorFromClass` "/Game/MyContent/FinalPro/BP_ShipSection_Rear.BP_ShipSection_Rear_C" _returnvalue "Undefined" "OverrideRootScale" null null))
  (`KismetArrayLibrary.Array_Add` _shipsegmentarray _returnvalue_3)
  (goto _label))

(fn `SetShipsMat`
  (params (BodyMat :type "MaterialInstance Object Reference") (AccentMat :type "MaterialInstance Object Reference"))
  (for _array_element (`self.ShipSegmentArray`)
    (bind _asbp_ship_section_master (cast `/Game/MyContent/FinalPro/BP_ShipSection_Master` _array_element))
    (`/Game/MyContent/FinalPro/BP_ShipSection_Master.ChangeMat` _asbp_ship_section_master BodyMat AccentMat)
    (`PrimitiveComponent.SetMaterial` (`self.Helm`) 0 BodyMat)
    (`PrimitiveComponent.SetMaterial` (`self.Connector`) 0 AccentMat)))

(fn `UserConstructionScript`)