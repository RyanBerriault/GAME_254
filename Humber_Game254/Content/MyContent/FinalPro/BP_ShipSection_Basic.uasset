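; BP_ShipSection_Basic is a ship section Blueprint whose materials can be swapped at runtime.
; A ChangeMat event takes a body material and an accent material, applying the first to MainBody and the second to both Connector and Accent, each on material slot 0.
; The BeginPlay, overlap and Tick events are disabled stubs, and the construction script only calls its parent.
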(event `self.ChangeMat`
  (params (NewBodyMat :type "MaterialInstance Object Reference") (NewAccentMat :type "MaterialInstance Object Reference"))
  (`PrimitiveComponent.SetMaterial` (`self.MainBody`) 0 NewBodyMat)
  (`PrimitiveComponent.SetMaterial` (`self.Connector`) 0 NewAccentMat)
  (`PrimitiveComponent.SetMaterial` (`self.Accent`) 0 NewAccentMat))

(fn `UserConstructionScript`
  (`parent.UserConstructionScript`))