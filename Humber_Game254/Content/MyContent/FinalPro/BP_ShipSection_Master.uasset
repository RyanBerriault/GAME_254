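; BP_ShipSection_Master is a ship section actor, apparently a base class for modular ship pieces that join end to end.
; Forward and rear connection point components expose their world transforms as attach points for other code.
; ChangeMat swaps the body material on MainBody and the accent material on Connector.
; AttachToPoint attaches the section to a given parent actor with keep-relative rules, and the event graph holds no logic.
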(fn `AttachToPoint`
  (params (ParentActor :type "Actor Object Reference"))
  (`self.K2_AttachToActor` ParentActor "None" "KeepRelative" "KeepRelative" "KeepRelative"))

(fn `ChangeMat`
  (params (NewBodyMat :type "MaterialInstance Object Reference") (NewAccentMat :type "MaterialInstance Object Reference"))
  (`PrimitiveComponent.SetMaterial` (`self.MainBody`) 0 NewBodyMat)
  (`PrimitiveComponent.SetMaterial` (`self.Connector`) 0 NewAccentMat))

(fn `GetFowardAttachTransform`
  (returns (Transform :type "Transform Structure"))
  (return (`SceneComponent.K2_GetComponentToWorld` (`self.ForwardConnectionPoint`))))

(fn `GetRearAttachTransform`
  (returns (Transform :type "Transform Structure"))
  (return (`SceneComponent.K2_GetComponentToWorld` (`self.RearConnectionPoint`))))

(fn `UserConstructionScript`)