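; BP_Fire is a fire actor that the player can toggle off and on with the E key.
; Overlapping its Box enables input from player 0 and sends CustomInteractionEventMessage(true) to the overlapping actor; leaving disables input and sends false.
; A FlipFlop on E alternately deactivates and reactivates the particle system and audio, starting with deactivation.
; The overlap events do not filter which actor triggers them.
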(event `self.Box.OnComponentBeginOverlap`
  (params (OverlappedComponent :type "PrimitiveComponent Object Reference") (OtherActor :type "Actor Object Reference") (OtherComp :type "PrimitiveComponent Object Reference") (OtherBodyIndex :type Integer) (bFromSweep :type Boolean) (SweepResult :type "HitResult Structure (by ref)"))
  (`self.EnableInput` (`GameplayStatics.GetPlayerController` 0))
  (message `/Game/MyContent/BP/BPI_Interactable.CustomInteractionEvent` OtherActor true))

(event `self.Box.OnComponentEndOverlap`
  (params (OverlappedComponent :type "PrimitiveComponent Object Reference") (OtherActor :type "Actor Object Reference") (OtherComp :type "PrimitiveComponent Object Reference") (OtherBodyIndex :type Integer))
  (`self.DisableInput` (`GameplayStatics.GetPlayerController` 0))
  (message `/Game/MyContent/BP/BPI_Interactable.CustomInteractionEvent` OtherActor false))

(event `Key|E`
  (params (Key :type "Key Structure"))
  (bind _particlesystemcomponent (`self.ParticleSystemComponent`))
  (bind _audio (`self.Audio`))
  (:`Pressed`
    (`/Engine/EditorBlueprintResources/StandardMacros.FlipFlop`
      (:`A`
        (`ActorComponent.Deactivate` _particlesystemcomponent)
        (`ActorComponent.Deactivate` _audio))
      (:`B`
        (`ActorComponent.Activate` _particlesystemcomponent true)
        (`ActorComponent.Activate` _audio true)))))

(fn `UserConstructionScript`)